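; PickupWeapon is a weapon Blueprint that grabs physics-simulating objects at range and carries them.
; A line trace along the Arrow's forward vector, up to PullDistance, finds a component for the PhysicsHandle to grab.
; Each tick, the handle's target moves to HeldObjectLocation, pulling the object there.
; KeepTriggerPulled selects hold-to-carry or a FlipFlop toggle between pickup and drop on trigger pulls.
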(event Custom|PickupObject
  (bind _arrow (Variables|Default|GetArrow))
  (bind _returnvalue (Transformation|GetWorldLocation _arrow))
  ;[1 1 1] pickup event
  (bind (_outhit _returnvalue_2) (Collision|LineTraceByChannel _returnvalue (+ _returnvalue (* (Math|Vector|GetForwardVector _arrow) (Variables|Default|GetPullDistance))) "TraceTypeQuery1" false 0 "None"))
  (if _returnvalue_2
    (if (Physics|IsSimulatingPhysics (.HitComponent (Collision|BreakHitResult _outhit)) "None")
      (Physics|Components|PhysicsHandle|GrabComponentatLocationwithRotation (Variables|Default|GetPhysicsHandle) (.HitComponent (Collision|BreakHitResult _outhit)) "None" (Transformation|GetWorldLocation (.HitComponent (Collision|BreakHitResult _outhit))) "0, 0, 0")
      (Variables|Default|SetIsHoldingObject? true))))

(event Custom|DropObject
  (Physics|Components|PhysicsHandle|ReleaseComponent (Variables|Default|GetPhysicsHandle))
  (Variables|Default|SetIsHoldingObject? false))

(event EventBeginPlay
  (|CallParentFunction) ; This node is disabled and will not be called.\nDrag off pins to build functionality.
)

(event Collision|EventActorBeginOverlap
  (params (OtherActor :type Actor%20Object%20Reference)))

(event EventTick
  (params (DeltaSeconds :type Float%20%28single-precision%29))
  (|CallParentFunction DeltaSeconds)
  (Physics|Components|PhysicsHandle|SetTargetLocation (Variables|Default|GetPhysicsHandle) (Transformation|GetWorldLocation (Variables|Default|GetHeldObjectLocation))))

(event EventTriggerPull
  (params (Player :type Jetpack%20Character%20Object%20Reference))
  (if (Variables|Default|GetKeepTriggerPulled?)
    (if (not (Variables|Default|GetIsHoldingObject?))
      (CallFunction|PickupObject))
    (else
      (Utilities|FlowControl|FlipFlop
        (:A
          (CallFunction|PickupObject))
        (:B
          (CallFunction|DropObject))))))

(event EventTriggerRelease
  (if (Variables|Default|GetKeepTriggerPulled?)
    (if true
      (CallFunction|DropObject))))

(fn ConstructionScript
  (|CallParentFunction))