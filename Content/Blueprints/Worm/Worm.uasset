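; Sand worm enemy that senses the player's steps on sand, hunts them and destroys them on hit while attacking.
; Tick runs a mental state machine from curious through hunting, attacking, diving and returning home, with adrenaline gating attacks.
; The physics head steers by clamped forces and leaps on solved ballistic arcs, with ground traces setting sand drag and gravity.
; Instanced body segments trail the head at fixed bone spacing.
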(event OnComponentBeginOverlap(WormHEAD)
  (params (OverlappedComponent :type Primitive%20Component%20Object%20Reference) (OtherActor :type Actor%20Object%20Reference) (OtherComp :type Primitive%20Component%20Object%20Reference) (OtherBodyIndex :type Integer) (bFromSweep :type Boolean) (SweepResult :type Hit%20Result%20Structure%20%28by%20ref%29))
  (if (> (Variables|CurrentStateData|GetTime%20In%20Current%20State) 0.5)
    (bind _returnvalue (Physics|GetPhysicsLinearVelocity (Variables|Default|GetWormHEAD) "None"))
    (if (< (.z _returnvalue) 0.0)
      (CallFunction|ChangeState "NewEnumerator5"))))

(event OnComponentEndOverlap(WormHEAD)
  (params (OverlappedComponent :type Primitive%20Component%20Object%20Reference) (OtherActor :type Actor%20Object%20Reference) (OtherComp :type Primitive%20Component%20Object%20Reference) (OtherBodyIndex :type Integer)))

(event OnComponentHit(WormHEAD)
  (params (HitComponent :type Primitive%20Component%20Object%20Reference) (OtherActor :type Actor%20Object%20Reference) (OtherComp :type Primitive%20Component%20Object%20Reference) (NormalImpulse :type Vector :default "0, 0, 0") (Hit :type Hit%20Result%20Structure%20%28by%20ref%29))
  (bind _asjetpack_character (Utilities|Casting|CastToJetpackCharacter OtherActor))
  (if (Utilities|Enum|Equal(Enum) (Variables|CurrentStateData|GetMental%20State) "NewEnumerator3")
    (Actor|DestroyActor _asjetpack_character)))

(event Custom|Player%20stepped%20on%20sand
  (params (Target :type Actor%20Object%20Reference) (Location :type Vector))
  (bind _wormhead (Variables|Default|GetWormHEAD))
  (bind _returnvalue (Transformation|GetWorldLocation _wormhead))
  (Utilities|IsValid (Variables|CurrentStateData|GetAttackTarget) ; Do we have a target?
    (:Is%20Valid
      (if (== (Variables|CurrentStateData|GetAttackTarget) Target) ; Is this our current target?
        (Variables|CurrentStateData|SetLast%20Sense%20Location Location :!label _label)
        (Variables|CurrentStateData|SetTime%20Since%20Last%20Sense 0.0)
        (if (or (Utilities|Enum|Equal(Enum) (Variables|CurrentStateData|GetMental%20State) "NewEnumerator0") (Utilities|Enum|Equal(Enum) (Variables|CurrentStateData|GetMental%20State) "NewEnumerator4"))
          (CallFunction|ChangeState "NewEnumerator1"))
        (elif (< (Math|Vector|VectorLengthSquared (- Location _returnvalue)) (Math|Vector|VectorLengthSquared (- _returnvalue (Variables|CurrentStateData|GetLast%20Sense%20Location)))) ; If this target is closer, make this the current target
          (Variables|CurrentStateData|SetAttackTarget Target :!label _label_2)
          (goto _label))))
    (:Is%20Not%20Valid
      (goto _label_2))))

(event Custom|Player%20stepped%20on%20crystls
  (params (Target :type Actor%20Object%20Reference))
  (if (== Target (Variables|CurrentStateData|GetAttackTarget))
    (Variables|CurrentStateData|SetAttackTarget 0)))

(event EventBeginPlay
  (Utilities|FlowControl|Sequence
    (:then_0
      (bind _asjetpack_character (Utilities|Casting|CastToJetpackCharacter (Game|GetPlayerCharacter 0)))
      (EventDispatchers|BindEventtoWalkedonSand _asjetpack_character (delegate Custom|Player%20stepped%20on%20sand))
      (EventDispatchers|BindEventtoWalkedonVibrationCrystals _asjetpack_character (delegate Custom|Player%20stepped%20on%20crystls)))
    (:then_1
      (Timeline|Move%20Segments Play
        (:Update
          (CallFunction|UpdateBody))))))

(event EventTick
  (params (DeltaSeconds :type Float%20%28single-precision%29))
  (bind _wormhead (Variables|Default|GetWormHEAD))
  (bind _attacktarget (Variables|CurrentStateData|GetAttackTarget))
  (bind _wormhead_2 (Variables|Default|GetWormHEAD))
  (bind _mental_state (Variables|CurrentStateData|GetMental%20State))
  (bind _last_sense_location (Variables|CurrentStateData|GetLast%20Sense%20Location))
  (bind _attacktarget_2 (Variables|CurrentStateData|GetAttackTarget))
  (bind _returnvalue (Transformation|GetWorldLocation _wormhead))
  (bind _returnvalue_2 (Transformation|GetWorldLocation _wormhead_2))
  (bind _returnvalue_3 (Transformation|GetActorLocation _attacktarget))
  (bind _returnvalue_4 (- _last_sense_location _returnvalue_2))
  (bind _returnvalue_5 (- _returnvalue _returnvalue_3))
  (CallFunction|Cooldowns DeltaSeconds)
  (CallFunction|FindGround)
  (CallFunction|SlowDowninSand DeltaSeconds)
  (Development|PrintString (Utilities|String|EnumtoString _mental_state))
  (switch Utilities|FlowControl|Switch|SwitchonWormMentalState _mental_state
    (:NewEnumerator1
      (if (> (Variables|CurrentStateData|GetTime%20In%20Current%20State) 12.0)
        (CallFunction|ChangeState "NewEnumerator4")
        (else
          (bind _is_close_enough_to_slow_down (CallFunction|CrawlTowards (+ (Variables|CurrentStateData|GetLast%20Sense%20Location) (Variables|CurrentStateData|GetRandom%20Offset)) DeltaSeconds 5e+02)) ; Crawl towards last known location
          (if _is_close_enough_to_slow_down
            (Variables|CurrentStateData|SetRandom%20Offset (* (Class|KismetMathLibrary|RandomUnitVectorinConeinRadians (Math|Vector|Normalize (Math|Vector|MakeVector (.x _returnvalue_4) (.y _returnvalue_4) -0.1)) 1.8e+02) 1e+03)))
          (Utilities|IsValid (Variables|CurrentStateData|GetAttackTarget) ; Does wormy sense a target?
            (:Is%20Valid
              (bind _target_is_heard (CallFunction|CanHearTarget (Variables|WormBehavior|GetHow%20close%20can%20hear%20target) (Variables|CurrentStateData|GetAttackTarget) 0.7))
              (if _target_is_heard
                (CallFunction|ChangeState "NewEnumerator2")))))))
    (:NewEnumerator2
      ;[1 1 1] Hunting
      (Utilities|IsValid (Variables|CurrentStateData|GetAttackTarget) ; Does wormy have a target?
        (:Is%20Valid
          (Utilities|InAir
            (:On%20/%20in%20ground
              (bind _is_close_enough_to_slow_down_2 (CallFunction|CrawlTowards (+ _returnvalue_3 (* (Math|Vector|Normalize (Math|Vector|MakeVector (.x _returnvalue_5) (.y _returnvalue_5) 0.0)) (* (Variables|WormBehavior|GetHow%20close%20to%20attack%20target) 0.9))) DeltaSeconds 2e+02)) ; Crawl towards last known location
              (if (not _is_close_enough_to_slow_down_2)
                (if (>= (Variables|CurrentStateData|GetCurrent%20Adrenaline%20Level) 0.8)
                  (bind _target_is_heard_2 (CallFunction|CanHearTarget (Variables|WormBehavior|GetHow%20close%20to%20attack%20target) (Variables|CurrentStateData|GetAttackTarget) 0.5))
                  (if _target_is_heard_2
                    ;[1 1 1] Attack
                    (CallFunction|JumpTowards (Transformation|GetActorLocation (Variables|CurrentStateData|GetAttackTarget)))
                    (CallFunction|ChangeState "NewEnumerator3")
                    (Variables|CurrentStateData|SetCurrent%20Adrenaline%20Level 0.0)
                    (Audio|Components|Audio|Play (Variables|Default|GetSoundAttack) 0.0)))))))
        (:Is%20Not%20Valid
          (CallFunction|ChangeState "NewEnumerator1"))))
    (:NewEnumerator3
      ;[1 1 1] Attacking
      (if (or (> (Variables|CurrentStateData|GetTime%20In%20Current%20State) 2.0) (not (Utilities|IsValid _attacktarget_2)))
        (CallFunction|ChangeState "NewEnumerator1")
        (CallFunction|CrawlTowards (Variables|CurrentStateData|GetLast%20Sense%20Location) DeltaSeconds 1e+02) ; Crawl towards last known location
        (else
          (CallFunction|CrawlTowards (Transformation|GetActorLocation _attacktarget_2) DeltaSeconds 1e+02) ; Crawl towards last known location
        )))
    (:NewEnumerator4
      ;[1 1 1] Returning Home
      (CallFunction|CrawlTowards (+ (Transformation|GetActorLocation) "0, 0,-600.000000") DeltaSeconds 5e+02) ; Crawl towards home
      (if (> (Variables|CurrentStateData|GetTime%20In%20Current%20State) 4.0)
        (CallFunction|ChangeState "NewEnumerator0")))
    (:NewEnumerator5
      ;[1 1 1] Diving
      (if (>= (Variables|CurrentStateData|GetTime%20In%20Current%20State) 1.0)
        (Development|PrintString "TOO LONG diving")
        (CallFunction|ChangeState "NewEnumerator1" :!label _label)
        (else
          (Utilities|IsValid (Variables|CurrentStateData|GetAttackTarget)
            (:Is%20Valid
              (bind _is_close_enough_to_slow_down_3 (CallFunction|CrawlTowards (+ (Variables|CurrentStateData|GetLast%20Sense%20Location) "0, 0,-800.000000") DeltaSeconds 5e+01)) ; Dive below target
              (if _is_close_enough_to_slow_down_3
                (goto _label)))
            (:Is%20Not%20Valid
              (bind _is_close_enough_to_slow_down_4 (CallFunction|CrawlTowards (+ (Transformation|GetWorldLocation (Variables|Default|GetWormHEAD)) "0,0.000000,-50.000000") DeltaSeconds 5e+01)) ; Dive straight down
              (if _is_close_enough_to_slow_down_4
                (goto _label)))))))))

(fn ConstructionScript
  (for _index (range 0 (- (Variables|WormBodyConfig|GetNumber%20of%20Segments) 1))
    (Components|InstancedStaticMesh|AddInstance (Variables|Default|GetWormBODY) (Math|Transform|MakeTransform (Math|Vector|MakeVector 0.0 0.0 (* _index (* (Variables|WormBodyConfig|GetBone%20Length) -1.0))) "0, 0, 0" "1,1,1"))))

(fn FindGround
  (bind _wormhead (Variables|Default|GetWormHEAD))
  (bind _returnvalue (Transformation|GetWorldLocation _wormhead))
  (bind (_outhit _returnvalue_2) (Class|KismetSystemLibrary|LineTraceSinglebyProfile (+ _returnvalue "0, 0,5000.000000") (+ _returnvalue "0, 0, 0") "SandLandscape" false 0 "ForOneFrame" true "(R=1.000000,G=0.000000,B=0.000000,A=1.000000)" "(R=0.085179,G=0.069809,B=0.182292,A=1.000000)"))
  (if _returnvalue_2 ; ground found above head
    (Variables|CurrentStateData|SetPhysicalState "NewEnumerator3")
    (bind _output_get (Variables|CurrentStateData|SetCurrent%20depth%20in%20sand (- (.Z (Math|Vector|BreakVector (.ImpactPoint (Collision|BreakHitResult _outhit)))) (.z (Transformation|GetWorldLocation (Variables|Default|GetWormHEAD))))))
    (else
      (bind (_outhit_2 _returnvalue_3) (Collision|LineTraceByChannel _returnvalue (+ _returnvalue "0.000000, 0,-100.000000") "TraceTypeQuery1" false 0 "ForOneFrame")) ; if not below the sand: shoot ray DOWN
      (if _returnvalue_3 ; found something
        (if (Utilities|Enum|Equal(Enum) (Variables|/Script/Engine.PhysicalMaterial|GetSurfaceType (.PhysMat (Collision|BreakHitResult _outhit_2))) "SurfaceType1")
          (Variables|CurrentStateData|SetPhysicalState "NewEnumerator1")
          (else
            (Variables|CurrentStateData|SetPhysicalState "NewEnumerator4")))
        (else
          (Variables|CurrentStateData|SetPhysicalState "NewEnumerator0"))))))

(fn CrawlTowards
  (params (Location :type Vector) (dt :type Float%20%28single-precision%29) (How%20close%20to%20start%20slowing :type Float%20%28single-precision%29))
  (bind _returnvalue (* How%20close%20to%20start%20slowing How%20close%20to%20start%20slowing))
  (bind _wormhead (Variables|Default|GetWormHEAD))
  (bind _wormhead_2 (Variables|Default|GetWormHEAD))
  (bind _max_speed (Variables|MovementPhysics|GetMAX%20SPEED))
  (bind _max_turn_force (Variables|MovementPhysics|GetMAX%20TURN%20FORCE))
  (bind _returnvalue_2 (Transformation|GetWorldLocation _wormhead_2))
  (bind _returnvalue_3 (- Location _returnvalue_2))
  (bind _returnvalue_4 (Math|Vector|VectorLengthSquared _returnvalue_3))
  (LocalVariables|SetIsCloseEnoughToSLOW (< _returnvalue_4 _returnvalue))
  (bind _returnvalue_5 (Physics|GetPhysicsLinearVelocity _wormhead "None"))
  (Physics|AddForce _wormhead (select (> (Math|Vector|VectorLength (- (* (Math|Vector|Normalize _returnvalue_3) (select (LocalVariables|GetIsCloseEnoughToSLOW) (* _max_speed (/ _returnvalue_4 _returnvalue)) _max_speed)) _returnvalue_5)) _max_turn_force) (* (Math|Vector|Normalize (- (* (Math|Vector|Normalize _returnvalue_3) (select (LocalVariables|GetIsCloseEnoughToSLOW) (* _max_speed (/ _returnvalue_4 _returnvalue)) _max_speed)) _returnvalue_5)) _max_turn_force) (- (* (Math|Vector|Normalize _returnvalue_3) (select (LocalVariables|GetIsCloseEnoughToSLOW) (* _max_speed (/ _returnvalue_4 _returnvalue)) _max_speed)) _returnvalue_5)) "None" true)
  (return (LocalVariables|GetIsCloseEnoughToSLOW)))

(fn JumpTowards
  (params (Location :type Vector))
  (bind _wormhead (Variables|Default|GetWormHEAD))
  (bind _max_jump_strength (Variables|MovementPhysics|GetMax%20Jump%20Strength))
  (bind _gravity (Variables|MovementPhysics|GetGravity))
  (bind _gravity_2 (Variables|MovementPhysics|GetGravity))
  (bind _gravity_3 (Variables|MovementPhysics|GetGravity))
  (bind _physicalstate (Variables|CurrentStateData|GetPhysicalState))
  (bind _returnvalue (Transformation|GetWorldLocation _wormhead))
  (bind _returnvalue_2 (Utilities|Select :Index _physicalstate :NewEnumerator0 0.0 :NewEnumerator1 1.0 :NewEnumerator3 1.0 :NewEnumerator4 0.8))
  (bind _returnvalue_3 (- Location _returnvalue))
  (bind _returnvalue_4 (* _max_jump_strength _returnvalue_2))
  (bind _returnvalue_5 (Math|Vector|MakeVector (.x _returnvalue_3) (.y _returnvalue_3) 0.0))
  (bind _returnvalue_6 (Math|Float|Square _returnvalue_4))
  (bind _returnvalue_7 (Math|Vector|VectorLengthSquared _returnvalue_5))
  (bind _returnvalue_8 (Math|Float|Square _returnvalue_6))
  (bind _returnvalue_9 (* (.z _returnvalue_3) _returnvalue_6 2.0))
  (bind _returnvalue_10 (Math|Float|Sqrt _returnvalue_7))
  (bind _returnvalue_11 (* _gravity _returnvalue_7))
  (bind _returnvalue_12 (+ _returnvalue_11 _returnvalue_9))
  (bind _returnvalue_13 (* _returnvalue_10 _gravity_3))
  (bind _returnvalue_14 (* _returnvalue_12 _gravity_2))
  (bind _returnvalue_15 (- _returnvalue_8 _returnvalue_14))
  (bind _returnvalue_16 (Math|Float|Sqrt _returnvalue_15))
  (if (not (< _returnvalue_15 0.0))
    (Physics|SetPhysicsLinearVelocity (Variables|Default|GetWormHEAD) "0, 0, 0" false "None")
    (Physics|AddImpulse (Variables|Default|GetWormHEAD) (Class|KismetMathLibrary|CreateVectorfromYawPitch (Class|KismetMathLibrary|DegAtan2 (.y _returnvalue_3) (.x _returnvalue_3)) (select (>= (Variables|CurrentStateData|GetCurrent%20Adrenaline%20Level) 0.95) (Class|KismetMathLibrary|DegAtan (/ (+ _returnvalue_6 _returnvalue_16) _returnvalue_13)) (Class|KismetMathLibrary|DegAtan (/ (- _returnvalue_6 _returnvalue_16) _returnvalue_13))) _returnvalue_4) "None" true)))

(fn UpdateBody
  (bind _wormbody (Variables|Default|GetWormBODY))
  (bind _returnvalue (Components|InstancedStaticMesh|GetInstanceCount _wormbody))
  (CallFunction|RotateHead)
  (Components|InstancedStaticMesh|UpdateInstanceTransform (Variables|Default|GetWormBODY) 0 (Math|Transform|MakeTransform (Transformation|GetWorldLocation (Variables|Default|GetWormHEAD)) "0, 0, 0" "1,1,1") true true true)
  (for _index (range 1 _returnvalue)
    (Components|InstancedStaticMesh|UpdateInstanceTransform _wormbody _index (Math|Transform|MakeTransform (+ (* (Math|Vector|Normalize (- (.location (.OutInstanceTransform (Components|InstancedStaticMesh|GetInstanceTransform _wormbody _index false))) (.location (.OutInstanceTransform (Components|InstancedStaticMesh|GetInstanceTransform _wormbody (- _index 1) false))))) (Variables|WormBodyConfig|GetBone%20Length)) (.location (.OutInstanceTransform (Components|InstancedStaticMesh|GetInstanceTransform _wormbody (- _index 1) false)))) "0, 0, 0" "1,1,1") false (== _index _returnvalue) true)))

(fn Cooldowns
  (params (dt :type Float%20%28single-precision%29))
  (Variables|CurrentStateData|SetTime%20In%20Current%20State (+ (Variables|CurrentStateData|GetTime%20In%20Current%20State) dt))
  (Variables|CurrentStateData|SetTime%20Since%20Last%20Sense (+ (Variables|CurrentStateData|GetTime%20Since%20Last%20Sense) dt))
  (Variables|CurrentStateData|SetCurrent%20Adrenaline%20Level (Math|Float|Clamp(Float) (+ (Variables|CurrentStateData|GetCurrent%20Adrenaline%20Level) (* dt (Utilities|Select :Index (Variables|CurrentStateData|GetMental%20State) :NewEnumerator0 -1.0 :NewEnumerator1 0.1 :NewEnumerator2 0.25 :NewEnumerator3 0.1 :NewEnumerator4 -0.25 :NewEnumerator5 0.15))))))

(fn ChangeState
  (params (New%20State :type WormMentalState%20Enum :default "NewEnumerator0"))
  (Variables|CurrentStateData|SetMental%20State New%20State)
  (Variables|CurrentStateData|SetTime%20In%20Current%20State 0.0))

(fn SlowDowninSand
  (params (dt :type Float%20%28single-precision%29))
  (bind _wormhead (Variables|Default|GetWormHEAD))
  (Physics|SetEnableGravity (Variables|Default|GetWormHEAD) (not (Utilities|Enum|Equal(Enum) (Variables|CurrentStateData|GetPhysicalState) "NewEnumerator3")))
  (if (Utilities|Enum|Equal(Enum) (Variables|CurrentStateData|GetPhysicalState) "NewEnumerator3")
    (bind _returnvalue (Physics|GetPhysicsLinearVelocity _wormhead "None"))
    (if (< (.Z (Math|Vector|BreakVector _returnvalue)) 0.0)
      (Physics|SetPhysicsLinearVelocity _wormhead (Math|Vector|MakeVector (.X (Math|Vector|BreakVector _returnvalue)) (.Y (Math|Vector|BreakVector _returnvalue)) (Math|Float|Clamp(Float) (+ (.Z (Math|Vector|BreakVector _returnvalue)) (* dt (Variables|MovementPhysics|GetSand%20Friction%20Multiplier))) -1e+06 0.0)) false "None"))))

(fn RotateHead
  (bind _wormhead (Variables|Default|GetWormHEAD))
  (bind _wormhead_2 (Variables|Default|GetWormHEAD))
  (bind _attacktarget (Variables|CurrentStateData|GetAttackTarget))
  (bind _returnvalue (Transformation|GetWorldRotation _wormhead_2))
  ;[1 1 1] Get rotation from movement
  (bind _returnvalue_2 (Physics|GetPhysicsLinearVelocity (Variables|Default|GetWormHEAD) "None"))
  (Utilities|IsValid _attacktarget
    (:Is%20Valid
      (Transformation|SetWorldRotation _wormhead (Math|Rotator|Lerp(Rotator) _returnvalue (Math|Rotator|Lerp(Rotator) (Math|Rotator|FindLookatRotation (Transformation|GetWorldLocation (Variables|Default|GetWormHEAD)) (Transformation|GetActorLocation _attacktarget)) (Math|Rotator|FindLookatRotation (Math|Vector|VectorZero) _returnvalue_2) 0.5 true) 0.1 true) false false))
    (:Is%20Not%20Valid
      (Transformation|SetWorldRotation _wormhead (Math|Rotator|Lerp(Rotator) _returnvalue (Math|Rotator|FindLookatRotation (Math|Vector|VectorZero) _returnvalue_2) 0.1 true) false false))))

(fn CanHearTarget
  (params (Distance :type Float%20%28single-precision%29) (Actor :type Actor%20Object%20Reference) (AlignmentThreshold :type Float%20%28single-precision%29))
  (bind _returnvalue (Transformation|GetActorLocation Actor))
  (bind _wormhead (Variables|Default|GetWormHEAD))
  (bind _returnvalue_2 (Transformation|GetWorldLocation _wormhead))
  (if (<= (Class|KismetMathLibrary|VectorDistanceSquared _returnvalue _returnvalue_2) (* Distance Distance)) ; Close enough?
    (bind _returnvalue_3 (Physics|GetPhysicsLinearVelocity (Variables|Default|GetWormHEAD) "None")) ; Is head pointed at it?
    (if (> (Math|Vector|DotProduct (Math|Vector|Normalize _returnvalue_3) (Math|Vector|Normalize (- _returnvalue _returnvalue_2))) AlignmentThreshold)
      (return true)
      (else
        (return false)))
    (else
      (return false))))